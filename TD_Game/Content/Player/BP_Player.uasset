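; BP_Player is the player Blueprint that handles input for highlighting grid tiles, apparently for island placement.
; When IA_placeIsland starts, it traces under the cursor on Visibility and passes the hit location to HighlightTile on the BP_GridManager found in the level, printing the result.
; IA_Move does nothing; disconnected leftover nodes would print a debug string and shift the pawn along Y.
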(event `EnhancedInput|/Game/Player/Input/Gameplay/IA_placeIsland`
  (params (ActionValue :type Boolean) (ElapsedSeconds :type "Float (double-precision)") (TriggeredSeconds :type "Float (double-precision)") (InputAction :type "InputAction Object Reference" :default "/Game/Player/Input/Gameplay/IA_placeIsland.IA_placeIsland"))
  (:`Started`
    (bind _returnvalue (`GameplayStatics.GetActorOfClass` "/Game/IslandsSystem/BP_GridManager.BP_GridManager_C"))
    (bind _returnvalue_2 (`GridManager.HighlightTile` _returnvalue (`.Location` (`GameplayStatics.BreakHitResult` (`PlayerController.GetHitResultUnderCursorByChannel` (`GameplayStatics.GetPlayerController` 0) "TraceTypeQuery1" true)))))
    (`KismetSystemLibrary.PrintString` (`KismetStringLibrary.Conv_IntPointToString` _returnvalue_2))))

(event `self.ReceiveTick`
  (params (DeltaSeconds :type "Float (single-precision)")))

(event `EnhancedInput|/Game/Player/Input/Gameplay/IA_Move`
  (params (ActionValue :type "Float (double-precision)") (ElapsedSeconds :type "Float (double-precision)") (TriggeredSeconds :type "Float (double-precision)") (InputAction :type "InputAction Object Reference" :default "/Game/Player/Input/Gameplay/IA_Move.IA_Move")))

(fn `UserConstructionScript`)